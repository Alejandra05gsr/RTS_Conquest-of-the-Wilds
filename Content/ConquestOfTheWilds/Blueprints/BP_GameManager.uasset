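; BP_GameManager is the manager Blueprint that creates the game HUD and connects it to buildings and units.
; On BeginPlay it adds WBP_HUD to the viewport, and the C key flip-flops mouse cursor visibility.
; Toggle events show the spawn or worker panel, then pass a valid building or mushroom to the HUD to bind worker/warrior spawning or lumberjack/miner job actions.
; A SetSelectedUnit function records the selected unit.
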(event `self.ReceiveBeginPlay`
  (bind _returnvalue (`|CreateWidget` "/Game/ConquestOfTheWilds/Blueprints/WidgetBP/WBP_HUD.WBP_HUD_C" null null))
  (bind _output_get (set `self.Wbp_HUD` _returnvalue))
  (`UserWidget.AddToViewport` _output_get 0))

(event `self.ReceiveActorOnClicked`
  (params (ButtonPressed :type "Key Structure")))

(event `Key|C`
  (params (Key :type "Key Structure"))
  ; Mostrar Cursor
  (:`Pressed`
    (`/Engine/EditorBlueprintResources/StandardMacros.FlipFlop`
      (:`A`
        (set `PlayerController.bShowMouseCursor` true (`GameplayStatics.GetPlayerController` 0)))
      (:`B`
        (set `PlayerController.bShowMouseCursor` false (`GameplayStatics.GetPlayerController` 0))))))

(event `Key|LeftMouseButton`
  (params (Key :type "Key Structure")))

(event `ToggleSpawnCanvas`
  (params (buliding :type "/Game/ConquestOfTheWilds/Blueprints/Builds/BP_MainBuild Object Reference"))
  (bind _wbp_hud (`self.Wbp_HUD`))
  ; SpawnCanvas
  (`/Game/ConquestOfTheWilds/Blueprints/WidgetBP/WBP_HUD.ShowSpawnPanel` _wbp_hud)
  (`/Engine/EditorBlueprintResources/StandardMacros.IsValid` buliding
    (:`Is Valid`
      (`/Game/ConquestOfTheWilds/Blueprints/WidgetBP/WBP_HUD.SpawnWorkerBindEvent` _wbp_hud buliding)
      (`/Game/ConquestOfTheWilds/Blueprints/WidgetBP/WBP_HUD.SpawnWarriorBindEvent` _wbp_hud buliding))))

(event `ToggleWorkerCanvas`
  (params (mushroom :type "/Game/ConquestOfTheWilds/Blueprints/CharactersBP/BP_Mushroom_RTS Object Reference"))
  (bind _wbp_hud (`self.Wbp_HUD`))
  ; WorkerCanvas
  (`/Game/ConquestOfTheWilds/Blueprints/WidgetBP/WBP_HUD.ShowWorkerPanel` _wbp_hud)
  (`/Engine/EditorBlueprintResources/StandardMacros.IsValid` mushroom
    (:`Is Valid`
      (`/Game/ConquestOfTheWilds/Blueprints/WidgetBP/WBP_HUD.WorkLeñadorBindEvent` _wbp_hud mushroom)
      (`/Game/ConquestOfTheWilds/Blueprints/WidgetBP/WBP_HUD.WorkMineroBindEvent` _wbp_hud mushroom))))

(fn `SetSelectedUnit`
  (params (NewUnit :type "CharacterRTS Object Reference"))
  (`self.SetSelectedUnit` NewUnit))

(fn `UserConstructionScript`)