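; PawnCreature_BP is a creature pawn that prototypes key-driven material highlight effects.
; BeginPlay creates and stores a dynamic instance of MI_PBR_PawnCreature, with no node in the graph assigning it to the mesh.
; F toggles the FresnelMask parameter on and off, and H starts a yoyo vector tween from a Color value.
; The mesh click event, construction script and leftover debug nodes do nothing.
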(event `self.ReceiveBeginPlay`
  (bind _returnvalue (`KismetMaterialLibrary.CreateDynamicMaterialInstance` "/Game/ConquestOfTheWilds/Materials/PawnCreature/MI_PBR_PawnCreature.MI_PBR_PawnCreature"))
  (set `self.DynamicMaterial` _returnvalue))

(event `self.SkeletalMesh.OnClicked`
  (params (TouchedComponent :type "PrimitiveComponent Object Reference") (ButtonPressed :type "Key Structure")))

(event `Key|F`
  (params (Key :type "Key Structure"))
  (:`Pressed`
    (`/Engine/EditorBlueprintResources/StandardMacros.FlipFlop`
      (:`A`
        (`KismetMaterialLibrary.SetScalarParameterValue` null (`self.fresnelMask`) 1.0))
      (:`B`
        (`KismetMaterialLibrary.SetScalarParameterValue` null (`self.fresnelMask`))))))

(event `Key|H`
  (params (Key :type "Key Structure"))
  (:`Pressed`
    (`FCTweenBPActionVector.TweenVector` (`self.color`) (0.0 0.0 0.0) 1.0 "InOutQuad" 0.0 0.0 0.0 0 0.0 true)))

(fn `UserConstructionScript`)