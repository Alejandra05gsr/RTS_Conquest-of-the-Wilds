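; Mushroom RTS character Blueprint that tests highlight and flicker effects on a runtime material, with click events disabled on BeginPlay.
; Box click, release or the Fresnel input drives a FlipFlop whose A output alone tweens the FresnelMask scalar toward IsNotPressed.
; The Flicker input runs a looping yoyo tween from the current tint toward TintColor, writing only on Yoyo to a parameter named None.
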(event `self.ReceiveBeginPlay`
  (set `PlayerController.bEnableClickEvents` false (`GameplayStatics.GetPlayerController` 0)))

(event `self.BoxCollision.OnClicked`
  (params (TouchedComponent :type "PrimitiveComponent Object Reference") (ButtonPressed :type "Key Structure"))
  (bind _runtimematerial (`/Game/ConquestOfTheWilds/Blueprints/BP_RuntimeMat.RuntimeMaterial` (`self.BP_RuntimeMat`)))
  (`/Engine/EditorBlueprintResources/StandardMacros.FlipFlop` :!label _label
    (:`A`
      (`KismetSystemLibrary.PrintString` "Fresnel ")
      (bind _returnvalue (`MaterialInstanceDynamic.K2_GetScalarParameterValue` _runtimematerial (`self.fresnelMask`)))
      (bind (_asynctaskproxy _value) (`FCTweenBPActionFloat.TweenFloat` _returnvalue (`KismetMathLibrary.Conv_BoolToDouble` (`self.isNotPressed`)) 0.3 "Linear")
        (:`ApplyEasing`
          (`MaterialInstanceDynamic.SetScalarParameterValue` _runtimematerial (`self.fresnelMask`) _value))))))

(event `InputAction|Fresnel`
  (params (Key :type "Key Structure"))
  (:`Pressed`
    (goto _label)))

(event `self.BoxCollision.OnReleased`
  (params (TouchedComponent :type "PrimitiveComponent Object Reference") (ButtonReleased :type "Key Structure"))
  (goto _label))

(event `InputAction|Flicker`
  (params (Key :type "Key Structure"))
  (bind _runtimematerial (`/Game/ConquestOfTheWilds/Blueprints/BP_RuntimeMat.RuntimeMaterial` (`self.BP_RuntimeMat`)))
  (:`Pressed`
    (bind _returnvalue (`MaterialInstanceDynamic.K2_GetVectorParameterValue` _runtimematerial (`self.tintParameter`)))
    (bind (_asynctaskproxy _value) (`FCTweenBPActionVector.TweenVector` (`KismetMathLibrary.Conv_LinearColorToVector` _returnvalue) (`KismetMathLibrary.Conv_LinearColorToVector` (`KismetMathLibrary.Conv_ColorToLinearColor` (`self.TintColor`))) 1.0 "InOutQuad" 0.0 0.0 0.0 4 0.0 true)
      (:`OnYoyo`
        (`MaterialInstanceDynamic.SetVectorParameterValue` _runtimematerial "None" (`KismetMathLibrary.Conv_VectorToLinearColor` _value))
        (`KismetSystemLibrary.PrintString` "Flicker")))))

(fn `UserConstructionScript`)