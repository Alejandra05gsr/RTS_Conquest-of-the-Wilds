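; Mushroom character for an RTS that gives click selection feedback and basic hit and death hooks through a runtime material.
; BeginPlay applies that material to the skeletal mesh; clicking its box under RTSController_BP tweens a Fresnel mask and sets FresnelActive.
; Flicker uses a vector tween for tint, and Die flags ABPT_Mushroom before calling Dither.
; Dither, MoveButton and CanvasMushroom are unfinished stubs.
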(event `self.ReceiveBeginPlay`
  (bind _bp_runtimemat (`self.BP_RuntimeMat`))
  (`/Game/ConquestOfTheWilds/Blueprints/BP_RuntimeMat.CreateRuntimeMaterial` _bp_runtimemat)
  (`/Game/ConquestOfTheWilds/Blueprints/BP_RuntimeMat.ApplyRuntimeMaterial` _bp_runtimemat (`|MakeArray` (`self.SkeletalMesh`) :!type "MeshComponent Object Reference")))

(event `self.BoxCollision.OnClicked`
  (params (TouchedComponent :type "PrimitiveComponent Object Reference") (ButtonPressed :type "Key Structure"))
  (cast `/Game/ConquestOfTheWilds/Blueprints/RTSController_BP` (`GameplayStatics.GetPlayerController` 0))
  (`self.Fresnel`))

(event `InitPosition`
  (bind _output_get (set `self.initPos` (`self.K2_GetActorLocation` self)))
  (`KismetSystemLibrary.PrintString` (`KismetStringLibrary.Conv_VectorToString` _output_get)))

(event `Fresnel`
  (bind _runtimematerial (`/Game/ConquestOfTheWilds/Blueprints/BP_RuntimeMat.RuntimeMaterial` (`self.BP_RuntimeMat`)))
  ; Fresnel
  (if (not (`self.fresnelActive`))
    (`KismetSystemLibrary.PrintString` "Fresnel")
    (bind _returnvalue (`MaterialInstanceDynamic.K2_GetScalarParameterValue` _runtimematerial (`self.fresnelMask`)))
    (bind (_asynctaskproxy _value) (`FCTweenBPActionFloat.TweenFloat` _returnvalue)
      (:`ApplyEasing`
        (`MaterialInstanceDynamic.SetScalarParameterValue` _runtimematerial (`self.fresnelMask`) _value)
        (set `self.fresnelActive` true)))))

(event `Flicker`
  (bind _tinitparameter (`self.tinitParameter`))
  (bind _runtimematerial (`/Game/ConquestOfTheWilds/Blueprints/BP_RuntimeMat.RuntimeMaterial` (`self.BP_RuntimeMat`)))
  ; Flicker
  (`KismetSystemLibrary.PrintString` "Flicker")
  (bind _returnvalue (`MaterialInstanceDynamic.K2_GetVectorParameterValue` _runtimematerial _tinitparameter))
  (bind (_asynctaskproxy _value) (`FCTweenBPActionVector.TweenVector` (`KismetMathLibrary.Conv_LinearColorToVector` _returnvalue) (`KismetMathLibrary.Conv_LinearColorToVector` (`KismetMathLibrary.Conv_ColorToLinearColor` (`self.tintColor`))) 0.5 "InOutQuad" 0.0 0.0 0.0 3 0.0 true)
    (:`OnComplete`
      (`MaterialInstanceDynamic.SetVectorParameterValue` _runtimematerial _tinitparameter (`KismetMathLibrary.Conv_VectorToLinearColor` _value))
      (`KismetSystemLibrary.PrintString` "end"))))

(event `Die`
  ; Die
  (bind _asabpt_mushroom (cast `/Game/ConquestOfTheWilds/Blueprints/AnimationBP/PlayerAnimation/ABPT_Mushroom` (`SkeletalMeshComponent.GetAnimInstance` (`self.SkeletalMesh`)))
    (:`then`
      (set `/Game/ConquestOfTheWilds/Blueprints/AnimationBP/PlayerAnimation/ABPT_Mushroom.activeValve` true _asabpt_mushroom))
    (:`CastFailed`
      _))
  (`self.Dither`))

(event `MoveButton`
  (if (`self.fresnelActive`)
    (if (`self.buttonMovePress`)
      _)))

(event `Dither`)

(event `CanvasMushroom`)

(fn `UserConstructionScript`)