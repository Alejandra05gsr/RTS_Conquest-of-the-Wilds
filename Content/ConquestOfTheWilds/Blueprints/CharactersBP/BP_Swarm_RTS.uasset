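; BP_Swarm_RTS is a swarm character that plays an attack montage near the player and dies when clicked or when L is pressed.
; Death plays a sound, sets the animation Blueprint's Dead flag and tweens a dither mask to zero on a runtime material.
; Tick triggers the attack on a distance check to the player pawn, whose threshold is zero, with a flag blocking replays until the montage completes.
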(event `self.ReceiveBeginPlay`
  (bind _bp_runtimemat (`self.BP_RuntimeMat`))
  (`/Game/ConquestOfTheWilds/Blueprints/BP_RuntimeMat.CreateRuntimeMaterial` _bp_runtimemat)
  (`/Game/ConquestOfTheWilds/Blueprints/BP_RuntimeMat.ApplyRuntimeMaterial` _bp_runtimemat (`|MakeArray` (`self.SkeletalMesh`) :!type "MeshComponent Object Reference")))

(event `Key|L`
  (params (Key :type "Key Structure"))
  ; Selected
  (:`Pressed`
    (`KismetSystemLibrary.PrintString` "Swarm" :!label _label)
    (`self.DieSound`)
    (`self.Die`)))

(event `self.BoxCollision.OnClicked`
  (params (TouchedComponent :type "PrimitiveComponent Object Reference") (ButtonPressed :type "Key Structure"))
  ; Selected
  (goto _label))

(event `Die`
  ; Die
  (bind _asabpt_swarm (cast `/Game/ConquestOfTheWilds/Blueprints/AnimationBP/PlayerAnimation/ABPT_Swarm` (`SkeletalMeshComponent.GetAnimInstance` (`self.SkeletalMesh`)))
    (:`then`
      (set `/Game/ConquestOfTheWilds/Blueprints/AnimationBP/PlayerAnimation/ABPT_Swarm.dead` true _asabpt_swarm))
    (:`CastFailed`
      _))
  (`self.Dither`))

(event `Dither`
  (bind _runtimematerial (`/Game/ConquestOfTheWilds/Blueprints/BP_RuntimeMat.RuntimeMaterial` (`self.BP_RuntimeMat`)))
  ; Dither
  (if (not (`self.ditherActive`))
    (bind _returnvalue (`MaterialInstanceDynamic.K2_GetScalarParameterValue` _runtimematerial (`self.DitherMask`)))
    (bind (_asynctaskproxy _value) (`FCTweenBPActionFloat.TweenFloat` _returnvalue 0.0 2.0)
      (:`ApplyEasing`
        (`MaterialInstanceDynamic.SetScalarParameterValue` _runtimematerial (`self.DitherMask`) _value)
        (set `self.ditherActive` true)))))

(event `self.ReceiveTick`
  (params (DeltaSeconds :type "Float (single-precision)"))
  ; Attack
  (if (<= (`self.GetDistanceTo` self (`GameplayStatics.GetPlayerPawn` 0)) 0.0)
    (if (not (`self.attacking`))
      (set `self.attacking` true)
      (`|PlayMontage` (`self.SkeletalMesh`) "/Game/ConquestOfTheWilds/Meshes/Swarm/AM_SwarmAttack.AM_SwarmAttack"
        (:`OnCompleted`
          (set `self.attacking` false))))))

(fn `DieSound`
  (`GameplayStatics.PlaySoundAtLocation` (`self.deathSound`) (`SceneComponent.K2_GetComponentLocation` (`self.BoxCollision`)) (struct) 1.0 1.0 0.0 null null null null))

(fn `UserConstructionScript`)