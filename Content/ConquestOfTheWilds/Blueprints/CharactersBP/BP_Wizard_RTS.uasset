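; BP_Wizard_RTS is a wizard character that wanders the map and dies when its capsule is clicked.
; From BeginPlay it sets up a runtime material and starts a looping AI move to random reachable nearby points, reissued on a delay without waiting for arrival.
; Death sets the Dead flag on the animation Blueprint, tweens a dither mask to fade the mesh and plays a sound.
; The collision-check and mushroom-attack events are empty stubs.
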(event `self.ReceiveBeginPlay`
  (bind _bp_runtimemat (`self.BP_RuntimeMat`))
  (`/Game/ConquestOfTheWilds/Blueprints/BP_RuntimeMat.CreateRuntimeMaterial` _bp_runtimemat)
  (`/Game/ConquestOfTheWilds/Blueprints/BP_RuntimeMat.ApplyRuntimeMaterial` _bp_runtimemat (`|MakeArray` (`self.Mesh`) :!type "MeshComponent Object Reference"))
  (`self.MoveToRandomPoint`))

(event `Die`
  ; Die
  (bind _asabpt_wizard (cast `/Game/ConquestOfTheWilds/Blueprints/AnimationBP/PlayerAnimation/ABPT_Wizard` (`SkeletalMeshComponent.GetAnimInstance` (`self.Mesh`)))
    (:`then`
      (set `/Game/ConquestOfTheWilds/Blueprints/AnimationBP/PlayerAnimation/ABPT_Wizard.dead` true _asabpt_wizard))
    (:`CastFailed`
      _))
  (`self.Dither`)
  (`self.DieSound`))

(event `Dither`
  (bind _runtimematerial (`/Game/ConquestOfTheWilds/Blueprints/BP_RuntimeMat.RuntimeMaterial` (`self.BP_RuntimeMat`)))
  ; Dither
  (if (not (`self.ditherActive`))
    (bind _returnvalue (`MaterialInstanceDynamic.K2_GetScalarParameterValue` _runtimematerial (`self.ditherMask`)))
    (bind (_asynctaskproxy _value) (`FCTweenBPActionFloat.TweenFloat` _returnvalue 0.0 2.0)
      (:`ApplyEasing`
        (`MaterialInstanceDynamic.SetScalarParameterValue` _runtimematerial (`self.ditherMask`) _value)
        (set `self.ditherActive` true)))))

(event `self.CapsuleCollision.OnClicked`
  (params (TouchedComponent :type "PrimitiveComponent Object Reference") (ButtonPressed :type "Key Structure"))
  (`self.Die`))

(event `MoveToRandomPoint`
  ; Movimiento aleatorio
  (`|AIMoveTo` self (`NavigationSystemV1.K2_GetRandomReachablePointInRadius` (`self.K2_GetActorLocation`) 3000.0 null null) null
    (:`then`
      (`KismetSystemLibrary.Delay` 5.0)
      (`self.MoveToRandomPoint`))))

(event `CheckCollisionPlayers`
  (if true
    _))

(event `AttackMushroom`)

(fn `DieSound`
  (`GameplayStatics.PlaySoundAtLocation` (`self.deathSound`) (`SceneComponent.K2_GetComponentLocation` (`self.CapsuleCollision`)) (struct) 1.0 1.0 0.0 null null null null))

(fn `UserConstructionScript`)