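; Actor component for CameraPawn_BP that pans the camera pawn from X and Y movement input.
; It caches its owning pawn on initialization, and BasicMovementController applies swept local offsets scaled by default speed and a modifier.
; A disable flag blocks movement, with separate branches for combined and single-axis input.
; A map-bounds check against min and max X and Y is present but disconnected, so it never runs.
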(event `InitComponent`
  (bind _ascamera_pawn_bp (cast `/Game/ConquestOfTheWilds/Blueprints/CameraBP/CameraPawn_BP` (`self.GetOwner`)))
  (set `self.CameraPawnRef` _ascamera_pawn_bp))

(event `self.ReceiveTick`
  (params (DeltaSeconds :type "Float (single-precision)")))

(fn `BasicMovementController`
  (params (MovValueX :type "Float (double-precision)") (MovValueY :type "Float (double-precision)"))
  (locals (MovValueXLocal :type "Float (double-precision)") (MovValueYLocal :type "Float (double-precision)"))
  (set `local.MovValueXLocal` MovValueX)
  (set `local.MovValueYLocal` MovValueY)
  (if (not (`self.disbaleCameraMov`))
    ; X and Y
    (if (and (!= (`local.MovValueXLocal`) 0.0) (!= (`local.MovValueYLocal`) 0.0))
      (`Actor.K2_AddActorLocalOffset` (`self.CameraPawnRef`) (+ (`KismetMathLibrary.MakeVector` (* (`local.MovValueXLocal`) (`self.DefaultMovementSpeed`) (`self.MovementSpeedModifier`))) (`KismetMathLibrary.MakeVector` 0.0 (* (`local.MovValueYLocal`) (`self.DefaultMovementSpeed`) (`self.MovementSpeedModifier`)))) true false)
      (else
        ; Only X
        (if (!= (`local.MovValueXLocal`) 0.0)
          (`Actor.K2_AddActorLocalOffset` (`self.CameraPawnRef`) (`KismetMathLibrary.MakeVector` (* (`local.MovValueXLocal`) (`self.DefaultMovementSpeed`) (`self.MovementSpeedModifier`))) true false)
          (else
            ; Only Y
            (if (!= (`local.MovValueYLocal`) 0.0)
              (`Actor.K2_AddActorLocalOffset` (`self.CameraPawnRef`) (`KismetMathLibrary.MakeVector` 0.0 (* (`local.MovValueYLocal`) (`self.DefaultMovementSpeed`) (`self.MovementSpeedModifier`))) true false))))))))