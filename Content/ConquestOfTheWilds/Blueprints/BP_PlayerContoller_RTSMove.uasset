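; Player controller for RTS-style camera movement in Conquest of the Wilds.
; On BeginPlay it shows the mouse cursor, enables click and hover events, and caches the CameraPawn_BP pawn and its CameraMovementComponent.
; The MoveForward and MoveRight axis inputs share one BasicMovementController call on that component, which does the movement work.
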(event `self.ReceiveBeginPlay`
  (`|ExecutionSequence`
    (:`then_0`
      (set `self.bShowMouseCursor` true)
      (set `self.bEnableClickEvents` true)
      (set `self.bEnableMouseOverEvents` true)
      (bind _ascamera_pawn_bp (cast `/Game/ConquestOfTheWilds/Blueprints/CameraBP/CameraPawn_BP` (`GameplayStatics.GetPlayerPawn` 0)))
      (bind _output_get (set `self.cameraPawnRef` _ascamera_pawn_bp))
      (set `self.cameraMovementRef` (`/Game/ConquestOfTheWilds/Blueprints/CameraBP/CameraPawn_BP.CameraMovementComponent` _output_get)))))

(event `InputAxis|MoveForward`
  (params (AxisValue :type "Float (single-precision)"))
  ; CameraMovement
  (`/Game/ConquestOfTheWilds/Blueprints/PlayerMovement_BP.BasicMovementController` (`self.CameraMovementRef`) AxisValue (stale `InputAxis|MoveRight` AxisValue) :!label _label))

(event `InputAxis|MoveRight`
  (params (AxisValue :type "Float (single-precision)"))
  ; CameraMovement
  (goto _label))

(fn `UserConstructionScript`)