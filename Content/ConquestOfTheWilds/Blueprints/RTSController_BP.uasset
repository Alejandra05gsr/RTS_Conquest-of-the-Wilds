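; RTS player controller for Conquest of the Wilds that sets up mouse interaction and passes camera movement input to the camera pawn.
; On BeginPlay it shows the cursor, enables click and mouse-over events, and caches the CameraPawn_BP and its CameraMovementComponent.
; The MoveForward and MoveRight axis events share one BasicMovementController call on that component, leaving the movement logic to it.
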(event `self.ReceiveBeginPlay`
  (`|ExecutionSequence`
    (:`then_0`
      (set `self.bShowMouseCursor` true)
      (set `self.bEnableClickEvents` true)
      (set `self.bEnableMouseOverEvents` true)
      (bind _ascamera_pawn_bp (cast `/Game/ConquestOfTheWilds/Blueprints/CameraPawn_BP` (`GameplayStatics.GetPlayerPawn` 0)))
      (bind _output_get (set `self.CameraPawnRef` _ascamera_pawn_bp))
      (set `self.CameraMovementRef` (`/Game/ConquestOfTheWilds/Blueprints/CameraPawn_BP.CameraMovementComponent` _output_get)))))

(event `Key|E`
  (params (Key :type "Key Structure")))

(event `InputAxis|MoveForward`
  (params (AxisValue :type "Float (single-precision)"))
  (`/Game/ConquestOfTheWilds/Blueprints/PlayerMovement_BP.BasicMovementController` (`self.CameraMovementRef`) AxisValue (stale `InputAxis|MoveRight` AxisValue) :!label _label))

(event `InputAxis|MoveRight`
  (params (AxisValue :type "Float (single-precision)"))
  (goto _label))

(fn `UserConstructionScript`)