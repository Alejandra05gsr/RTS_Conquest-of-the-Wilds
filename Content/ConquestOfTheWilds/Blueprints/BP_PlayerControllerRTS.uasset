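; RTS player controller that shows the cursor, drives the camera pawn and issues right-click moves.
; BeginPlay caches the pawn's CameraMovementComponent, which both movement axes feed within limits, passing the same value as X and Y.
; Right-click calls SimpleMoveToLocation at the cursor hit, and AddSelectedUnits stores unique units.
; Left-press HUD handlers and mushroom spawning are disconnected, so Tick's hold message lacks its trigger here; GrabSelectedUnits is empty.
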(event `self.ReceiveBeginPlay`
  (`|ExecutionSequence`
    (:`then_0`
      (set `self.bShowMouseCursor` true)
      (set `self.bEnableClickEvents` true)
      (set `self.bEnableMouseOverEvents` true)
      (bind _ascamera_pawn_bp (cast `/Game/ConquestOfTheWilds/Blueprints/CameraBP/CameraPawn_BP` (`GameplayStatics.GetPlayerPawn` 0)))
      (bind _output_get (set `self.CameraPawnRef` _ascamera_pawn_bp))
      (set `self.CameraMovementRef` (`/Game/ConquestOfTheWilds/Blueprints/CameraBP/CameraPawn_BP.CameraMovementComponent` _output_get)))))

(event `InputAxis|MoveForward`
  (params (AxisValue :type "Float (single-precision)"))
  ; CameraMovement
  (if (<= AxisValue (`self.limitTop`))
    (if (>= AxisValue (`self.limitDown`))
      (`/Game/ConquestOfTheWilds/Blueprints/PlayerMovement_BP.BasicMovementController` (`self.CameraMovementRef`) AxisValue (stale `InputAxis|MoveRight` AxisValue) :!label _label))))

(event `InputAxis|MoveRight`
  (params (AxisValue :type "Float (single-precision)"))
  ; CameraMovement
  (if (<= AxisValue (`self.limitRight`))
    (if (>= AxisValue (`self.limitLeft`))
      (goto _label))))

(event `self.ReceiveTick`
  (params (DeltaSeconds :type "Float (single-precision)"))
  (if (`self.isLeftMousePressed`)
    (message `/Game/ConquestOfTheWilds/Blueprints/BP_Interface.MouseHold` (`self.GetHUD`))))

(event `Key|LeftMouseButton`
  (params (Key :type "Key Structure")))

(event `Movement`)

(event `Key|RightMouseButton`
  (params (Key :type "Key Structure"))
  (:`Pressed`
    (`AIBlueprintHelperLibrary.SimpleMoveToLocation` null (`.Location` (`GameplayStatics.BreakHitResult` (`self.GetHitResultUnderCursorByChannel` "TraceTypeQuery1"))))))

(fn `AddSelectedUnits`
  (params (NewUnit :type "CharacterRTS Object Reference"))
  (`KismetArrayLibrary.Array_AddUnique` (`self.selectedUnits`) NewUnit))

(fn `GrabSelectedUnits`
  (returns (Units :type "Array of CharacterRTS Object Reference"))
  (return))

(fn `UserConstructionScript`)